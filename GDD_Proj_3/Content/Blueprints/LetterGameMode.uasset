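; LetterGameMode is a game mode for a local multiplayer word game that creates extra players and scatters a random target word's letters.
; BeginPlay picks the word and splits it into a text array.
; Tick calls SpawnLetter until the letter cap, spawning RandomLetter_BP actors at target points.
; Used-index lists aim to prevent repeats and reset when full, but random values re-roll between check and use.
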(event EventBeginPlay
  (Class|GameplayStatics|CreatePlayer 1 false)
  (Class|GameplayStatics|CreatePlayer 2 false)
  (Class|GameplayStatics|CreatePlayer 3 false)
  (Class|GameplayStatics|CreatePlayer 4 false)
  (bind _output_get (Variables|Default|SetTargetWord (Utilities|Array|Get(acopy) (Variables|Default|GetTargetWords) (Math|Random|RandomIntegerinRange 0 5))))
  (for _array_element (Utilities|String|GetCharacterArrayfromString (Utilities|String|ToString(Text) _output_get))
    (Utilities|Array|Add (Variables|Default|GetTextArr) (Utilities|Text|ToText(String) _array_element))))

(event EventTick
  (params (DeltaSeconds :type Float%20%28single-precision%29))
  (if (< (Variables|Default|GetLetterCount) (Variables|Default|GetMaxLetters))
    (CallFunction|SpawnLetter)))

(fn ConstructionScript)

(fn SpawnLetter
  (bind _returnvalue (Math|Random|RandomIntegerinRange 0 9))
  (bind _textarr (Variables|Default|GetTextArr))
  (bind _returnvalue_2 (Utilities|Array|Length _textarr))
  (bind _returnvalue_3 (- _returnvalue_2 1))
  (bind _returnvalue_4 (Math|Random|RandomIntegerinRange 0 _returnvalue_3))
  (if (Utilities|Array|ContainsItem (Variables|Default|GetRandomTextNums) _returnvalue_4)
    _
    (else
      (bind _output_get (Variables|Default|SetRandomNum _returnvalue_4))
      (Utilities|Array|Add (Variables|Default|GetRandomTextNums) _output_get)
      (if (Utilities|Array|ContainsItem (Variables|Default|GetRandomLocNums) _returnvalue)
        _
        (else
          (Utilities|Array|Add (Variables|Default|GetRandomLocNums) _returnvalue)
          (Game|SpawnActorfromClass "/Game/Blueprints/RandomLetter_BP.RandomLetter_BP_C" (Math|Transform|MakeTransform (Transformation|GetActorLocation (Utilities|Array|Get(acopy) (Variables|Default|GetTargetPointArray) _returnvalue)) "0, 0, 0" "1,1,1") "DontSpawnIfColliding" 0 (Variables|Default|GetTextArr) (Variables|Default|GetRandomNum))
          (Math|Integer|IncrementInt (Variables|Default|GetLetterCount)
            (:%20%20
              _))))))
  (if (== (Utilities|Array|Length (Variables|Default|GetRandomTextNums)) (Utilities|Array|Length (Variables|Default|GetTextArr)))
    (Utilities|Array|Clear (Variables|Default|GetRandomTextNums)))
  (if (== (Utilities|Array|Length (Variables|Default|GetRandomLocNums)) 10)
    (Utilities|Array|Clear (Variables|Default|GetRandomLocNums))))