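; Player platformer for a letter-collecting word game: moves and jumps by physics velocity on per-player keys, and restarts the game when destroyed.
; Overlapped letters join a collection and grow the attached FragTrail, which fires the first or last letter on key press.
; Tick rebuilds the collected string, opening Menu when it matches the game mode's target word.
; Ability keys spend matching words once each for score; ability effects are absent.
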(event EventBeginPlay
  ;[1 1 1] Enabling Input
  (if (Variables|Default|GetDebug)
    (Input|EnableInput (Game|GetPlayerController 0))
    ;[1 1 1] Cache the initial frag trail
    (bind _asfrag_trail (Utilities|Casting|CastToFragTrail (Utilities|Array|Get(acopy) (Actor|GetAttachedActors)))
      (:then
        (Variables|Default|SetFragTrail _asfrag_trail)
        (Variables|/Game/Trail/FragTrail.FragTrail_C|SetParentPlatformer (Variables|Default|GetFragTrail) self))
      (:CastFailed
        (Development|PrintText "Hello")))
    (else
      (Input|EnableInput (Game|GetPlayerController (Variables|Default|GetPlayerNum))))))

(event EventTick
  (params (DeltaSeconds :type Float%20%28single-precision%29))
  (bind _hitbox (Variables|Default|GetHitbox))
  (bind _returnvalue (Transformation|GetComponentVelocity _hitbox))
  (bind (_x _y _z) (Math|Vector|BreakVector _returnvalue))
  (Variables|Default|SetdeltaTime DeltaSeconds)
  ;[1 1 1] Update Collection String
  (CallFunction|CleanCollection)
  (Variables|Default|SetCollectionString "")
  (for _array_element (Variables|Default|GetLetterCollection)
    (bind _output_get (Variables|Default|SetCollectionString (Utilities|String|Append (Variables|Default|GetCollectionString) (Utilities|String|ToString(Text) _array_element)))))
  (bind _asletter_game_mode (Utilities|Casting|CastToLetterGameMode (Game|GetGameMode)))
  (if (Utilities|Enum|Equal(Enum) (Utilities|String|ToString(Text) (Variables|/Game/Blueprints/LetterGameMode.LetterGameMode_C|GetTargetWord _asletter_game_mode)) _output_get)
    (Game|OpenLevel(byName) "Menu")
    (else
      ;[1 1 1] Deciding whether to Reset the Jump Timer
      (if (== (Math|Float|Round (.Z (Math|Vector|BreakVector (Transformation|GetComponentVelocity (Variables|Default|GetHitbox))))) 0)
        (Variables|Default|SetjumpTimer 1.0))
      ;[1 1 1] Deciding whether make the Platformer Jump
      (if (and (Variables|Default|Getjumping) (> (Variables|Default|GetjumpTimer) 0.0))
        ;[1 1 1] Making the Platformer Jump
        (Physics|SetPhysicsLinearVelocity (Variables|Default|GetHitbox) (Math|Vector|MakeVector 0.0 0.0 (* (Variables|Default|GetjumpHeight) (Variables|Default|GetjumpTimer))) true "None")
        (Variables|Default|SetjumpTimer (- (Variables|Default|GetjumpTimer) (* (Variables|Default|GetdeltaTime) 6.0))))
      ;[1 1 1] Deciding whether to Move the Platformer Horizontally
      (if (Math|Boolean|NotEqual(Boolean) (Variables|Default|GetmovingRight) (Variables|Default|GetmovingLeft))
        (if (Variables|Default|GetmovingRight)
          ;[1 1 1] Moving the Platformer Right
          (Physics|SetPhysicsLinearVelocity (Variables|Default|GetHitbox) (Math|Vector|MakeVector 0.0 (* (Variables|Default|Getacceleration) (Variables|Default|GetdeltaTime)) 0.0) true "None")
          (else
            ;[1 1 1] Moving the Platformer Left
            (Physics|SetPhysicsLinearVelocity (Variables|Default|GetHitbox) (Math|Vector|MakeVector 0.0 (* (Variables|Default|Getacceleration) (Variables|Default|GetdeltaTime) -1.0) 0.0) true "None")))
        ;[1 1 1] Deciding whether to Limit the Y Speed
        (if (> (Math|Float|Absolute(Float) (.Y (Math|Vector|BreakVector (Transformation|GetComponentVelocity (Variables|Default|GetHitbox))))) (Variables|Default|GetmaxSpeed))
          ;[1 1 1] Limiting the Y Speed of the Platformer
          (Physics|SetPhysicsLinearVelocity (Variables|Default|GetHitbox) (Math|Vector|MakeVector _x (* (/ _y (Math|Float|Absolute(Float) _y)) (Variables|Default|GetmaxSpeed)) _z) false "None"))))))

(event EventDestroyed
  ;[1 1 1] Restart when one player dies
  (Class|GameMode|RestartGame (Game|GetGameMode)))

(event Collision|EventActorBeginOverlap
  (params (OtherActor :type Actor%20Object%20Reference))
  ;[1 1 1] Collecting a letter
  (if (Variables|/Game/Trail/FragTrail.FragTrail_C|Getspawned (Variables|Default|GetFragTrail)) ; Keeps us from collecting 2 at once
    (bind _asrandom_letter_bp (Utilities|Casting|CastToRandomLetter_BP OtherActor))
    (if (not (Utilities|Array|ContainsItem (Variables|Default|GetLetterCollection) (Variables|/Script/Engine.TextRenderComponent|GetText (Variables|/Game/Blueprints/RandomLetter_BP.RandomLetter_BP_C|GetTextRender _asrandom_letter_bp))))
      (Utilities|Array|Add (Variables|Default|GetLetterCollection) (Variables|/Script/Engine.TextRenderComponent|GetText (Variables|/Game/Blueprints/RandomLetter_BP.RandomLetter_BP_C|GetTextRender _asrandom_letter_bp)))
      (Default|LetterGrowTrail2 (Variables|Default|GetFragTrail))
      (Actor|DestroyActor _asrandom_letter_bp))))

(event Input|KeyboardEvents|AnyKey
  (params (Key :type Key%20Structure :default "AnyKey"))
  ;[1 1 1] Listening for the Ability 3 Key
  (:Pressed
    (if (or (== Key (Variables|Input|GetabilityKey3)) (== Key (Variables|DebugInput|GetdebugAbilityKey3)))
      (if (Utilities|Enum|Equal(Enum) (Variables|Default|GetCollectionString) (Variables|AbilityStrings|GetabilityString3))
        (if (not (Variables|Default|GetfroznUsed))
          (Variables|Default|SetfroznUsed true)
          (Utilities|Array|Clear (Variables|Default|GetLetterCollection))
          (Variables|Default|Setscore (+ (Variables|Default|Getscore) 5)))))))

(event Input|KeyboardEvents|AnyKey
  (params (Key :type Key%20Structure :default "AnyKey"))
  (bind _jumpkey (Variables|Input|GetjumpKey))
  (bind _debugjumpkey (Variables|DebugInput|GetdebugJumpKey))
  (bind _returnvalue (== Key _debugjumpkey))
  (bind _returnvalue_2 (== Key _jumpkey))
  (bind _returnvalue_3 (or _returnvalue_2 _returnvalue))
  ;[1 1 1] Listening for the Jump Key
  (:Pressed
    (if _returnvalue_3
      (Variables|Default|Setjumping true)))
  (:Released
    (if _returnvalue_3
      (Variables|Default|Setjumping false)
      (Variables|Default|SetjumpTimer 0.0))))

(event Input|KeyboardEvents|AnyKey
  (params (Key :type Key%20Structure :default "AnyKey"))
  (bind _moverightkey (Variables|Input|GetmoveRightKey))
  (bind _debugrightkey (Variables|DebugInput|GetdebugRightKey))
  (bind _returnvalue (== Key _moverightkey))
  (bind _returnvalue_2 (== Key _debugrightkey))
  (bind _returnvalue_3 (or _returnvalue _returnvalue_2))
  ;[1 1 1] Listening for the Move Right Key
  (:Pressed
    (if _returnvalue_3
      (Variables|Default|SetmovingRight true)))
  (:Released
    (if _returnvalue_3
      (Variables|Default|SetmovingRight false))))

(event Input|KeyboardEvents|AnyKey
  (params (Key :type Key%20Structure :default "AnyKey"))
  ;[1 1 1] Listening for the Ability 4 Key
  (:Pressed
    (if (or (== Key (Variables|Input|GetabilityKey4)) (== Key (Variables|DebugInput|GetdebugAbilityKey4)))
      (if (Utilities|Enum|Equal(Enum) (Variables|Default|GetCollectionString) (Variables|AbilityStrings|GetabilityString4))
        (if (not (Variables|Default|GetxpldeUsed))
          (Variables|Default|SetxpldeUsed true)
          (Utilities|Array|Clear (Variables|Default|GetLetterCollection))
          (Variables|Default|Setscore (+ (Variables|Default|Getscore) 5)))))))

(event Input|KeyboardEvents|AnyKey
  (params (Key :type Key%20Structure :default "AnyKey"))
  (bind _lettercollection (Variables|Default|GetLetterCollection))
  (bind _returnvalue (Utilities|Array|Length _lettercollection))
  (bind _returnvalue_2 (- _returnvalue 1))
  ;[1 1 1] Removes last letter from collection
  (:Pressed
    (if (> (Utilities|Array|Length (Variables|Default|GetLetterCollection)) 0)
      (if (or (== Key (Variables|Input|GetlastLetterKey)) (== Key (Variables|DebugInput|GetdebugLastLetterKey)))
        (Default|FireJumbo (Variables|Default|GetFragTrail) true (Utilities|Array|Get(acopy) _lettercollection _returnvalue_2))
        (Utilities|Array|RemoveIndex _lettercollection _returnvalue_2)))))

(event Input|KeyboardEvents|AnyKey
  (params (Key :type Key%20Structure :default "AnyKey"))
  (bind _lettercollection (Variables|Default|GetLetterCollection))
  ;[1 1 1] Removes first letter from collection
  (:Pressed
    (if (> (Utilities|Array|Length (Variables|Default|GetLetterCollection)) 0)
      (if (or (== Key (Variables|Input|GetfirstLetterKey)) (== Key (Variables|DebugInput|GetdebugFirstLetterKey)))
        (Default|FireJumbo (Variables|Default|GetFragTrail) false (Utilities|Array|Get(acopy) _lettercollection))
        (Utilities|Array|RemoveIndex _lettercollection)))))

(event Input|KeyboardEvents|AnyKey
  (params (Key :type Key%20Structure :default "AnyKey"))
  (bind _moveleftkey (Variables|Input|GetmoveLeftKey))
  (bind _debugleftkey (Variables|DebugInput|GetdebugLeftKey))
  (bind _returnvalue (== Key _moveleftkey))
  (bind _returnvalue_2 (== Key _debugleftkey))
  (bind _returnvalue_3 (or _returnvalue _returnvalue_2))
  ;[1 1 1] Listening for the Move Left Key
  (:Pressed
    (if _returnvalue_3
      (Variables|Default|SetmovingLeft true)))
  (:Released
    (if _returnvalue_3
      (Variables|Default|SetmovingLeft false))))

(event Input|KeyboardEvents|AnyKey
  (params (Key :type Key%20Structure :default "AnyKey"))
  ;[1 1 1] Listening for the Ability 1 Key
  (:Pressed
    (if (or (== Key (Variables|Input|GetabilityKey1)) (== Key (Variables|DebugInput|GetdebugAbilityKey1)))
      (if (Utilities|Enum|Equal(Enum) (Variables|Default|GetCollectionString) (Variables|AbilityStrings|GetabilityString1))
        (if (not (Variables|Default|GetquickUsed))
          (Variables|Default|SetquickUsed true)
          (Utilities|Array|Clear (Variables|Default|GetLetterCollection))
          (Variables|Default|Setscore (+ (Variables|Default|Getscore) 5)))))))

(event Input|KeyboardEvents|AnyKey
  (params (Key :type Key%20Structure :default "AnyKey"))
  ;[1 1 1] Listening for the Ability 2 Key
  (:Pressed
    (if (or (== Key (Variables|Input|GetabilityKey2)) (== Key (Variables|DebugInput|GetdebugAbilityKey2)))
      (if (Utilities|Enum|Equal(Enum) (Variables|Default|GetCollectionString) (Variables|AbilityStrings|GetabilityString2))
        (if (not (Variables|Default|GetjumboUsed))
          (Variables|Default|SetjumboUsed true)
          (Utilities|Array|Clear (Variables|Default|GetLetterCollection))
          (Variables|Default|Setscore (+ (Variables|Default|Getscore) 5)))))))

(fn ConstructionScript
  (bind _asletter_game_mode (Utilities|Casting|CastToLetterGameMode (Game|GetGameMode)))
  (Variables|Default|SetCollectionString (Utilities|String|ToString(Text) (Variables|/Game/Blueprints/LetterGameMode.LetterGameMode_C|GetTargetWord _asletter_game_mode))))

(fn InLetterCollection
  (params (letterString :type String))
  ;[1 1 1] FOR all letters in the passed string...
  (for _array_element (Utilities|String|GetCharacterArrayfromString letterString)
    ;[1 1 1] If the next letter in the array was not found, return false (all letters are NOT in collection)
    (Development|PrintString "loop")
    (if (== -1 (Utilities|Array|FindItem (Variables|Default|GetLetterCollection) (Utilities|Text|ToText(String) _array_element)))
      (return false)))
  (Development|PrintString "end")
  (return true) ; If the FOR loop completed, return true (all letters are in collection)
)

(fn CleanCollection
  ;[1 1 1] IF the collection is not empty...
  (if (> (Utilities|Array|Length (Variables|Default|GetLetterCollection)) 0)
    ;[1 1 1] FOR every letter in the collection (traversing through collection backwards)
    (for _index (range (* (- (Utilities|Array|Length (Variables|Default|GetLetterCollection)) 1) -1) 0)
      ;[1 1 1] IF the current letter is nothing, delete the letter
      (if (Utilities|Text|TextIsEmpty (Class|KismetTextLibrary|TextTrimPrecedingandTrailing (Utilities|Array|Get(acopy) (Variables|Default|GetLetterCollection) (Math|Integer|Absolute(Integer) _index))))
        (Utilities|Array|RemoveIndex (Variables|Default|GetLetterCollection) (Math|Integer|Absolute(Integer) _index))))))