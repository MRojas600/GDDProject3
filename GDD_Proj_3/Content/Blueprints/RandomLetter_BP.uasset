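; RandomLetter is a timed pickup actor that shows a random letter and calls LetterGrowTrail on an overlapping FragTrail.
; Construction picks the letter and lifespan, but rolls OriginalLifeSpan separately, so it can differ from the actual lifespan.
; Tick recolors the text in four stages from the remaining-to-original lifespan ratio.
; Any box overlap destroys the actor, and destruction decrements LetterCount on LetterGameMode.
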(event OnComponentBeginOverlap(Box)
  (params (OverlappedComponent :type Primitive%20Component%20Object%20Reference) (OtherActor :type Actor%20Object%20Reference) (OtherComp :type Primitive%20Component%20Object%20Reference) (OtherBodyIndex :type Integer) (bFromSweep :type Boolean) (SweepResult :type Hit%20Result%20Structure%20%28by%20ref%29))
  (Utilities|FlowControl|Sequence
    (:then_0
      (bind _asfrag_trail (Utilities|Casting|CastToFragTrail OtherActor))
      (Default|LetterGrowTrail _asfrag_trail))
    (:then_1
      (Actor|DestroyActor))))

(event EventBeginPlay)

(event EventTick
  (params (DeltaSeconds :type Float%20%28single-precision%29))
  (bind _returnvalue (Actor|GetLifeSpan))
  (bind _originallifespan (Variables|Default|GetOriginalLifeSpan))
  (bind _returnvalue_2 (/ _returnvalue _originallifespan))
  ;[1 1 1] Bases the color of the text off it's lifespan
  (if (>= _returnvalue_2 0.75)
    (Rendering|Components|TextRender|SetTextRenderColor (Variables|Default|GetTextRender) (Math|Conversions|ToColor(LinearColor) (Utilities|Array|Get(acopy) (Variables|Default|GetColorArray))))
    (elif (and (>= _returnvalue_2 0.5) (< _returnvalue_2 0.75))
      (Rendering|Components|TextRender|SetTextRenderColor (Variables|Default|GetTextRender) (Math|Conversions|ToColor(LinearColor) (Utilities|Array|Get(acopy) (Variables|Default|GetColorArray) 1)))
      (elif (and (>= _returnvalue_2 0.25) (< _returnvalue_2 0.5))
        (Rendering|Components|TextRender|SetTextRenderColor (Variables|Default|GetTextRender) (Math|Conversions|ToColor(LinearColor) (Utilities|Array|Get(acopy) (Variables|Default|GetColorArray) 2)))
        (elif (and (> _returnvalue_2 0.0) (< _returnvalue_2 0.25))
          (Rendering|Components|TextRender|SetTextRenderColor (Variables|Default|GetTextRender) (Math|Conversions|ToColor(LinearColor) (Utilities|Array|Get(acopy) (Variables|Default|GetColorArray) 3))))))))

(event EventDestroyed
  (bind _asletter_game_mode (Utilities|Casting|CastToLetterGameMode (Game|GetGameMode)))
  (Math|Integer|DecrementInt (Variables|/Game/Blueprints/LetterGameMode.LetterGameMode_C|GetLetterCount _asletter_game_mode)))

(fn ConstructionScript
  (bind _returnvalue (Math|Random|RandomFloatinRange 11.0 15.0))
  (Rendering|Components|TextRender|SetText (Variables|Default|GetTextRender) (Utilities|Array|Get(acopy) (Variables|Default|GetTextArray) (Math|Random|RandomIntegerinRange 0 25)))
  (Actor|SetLifeSpan _returnvalue)
  (Variables|Default|SetOriginalLifeSpan _returnvalue))